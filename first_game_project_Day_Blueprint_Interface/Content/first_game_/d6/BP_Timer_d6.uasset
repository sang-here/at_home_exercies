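; Practice timer Blueprint that prints an MM:SS clock to the screen, running at ten times real speed.
; Tick accumulates scaled DeltaSeconds into TotalDeltaSeconds, then derives minutes by division by 60 and seconds by modulo.
; The FloatToStr00 helper floors each value and zero-pads it to two digits.
; Disconnected earlier attempts remain in the graph, including a branch-heavy version built without the helper function.
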(event EventTick
  (params (DeltaSeconds :type Float%20%28single-precision%29))
  ;[0.15 0.15 0.15 0.5] 미리 만드는 함수로 함수의 귀여움을 경험하며 00:00 시계를 깔끔하게 만들기
  (bind _output_get (Variables|Default|SettotalDeltaSeconds (+ (Variables|Default|GettotalDeltaSeconds) (* DeltaSeconds 1e+01))))
  (Development|PrintString (Utilities|String|Append (CallFunction|FloattoStr00 (/ _output_get 6e+01)) ":" (CallFunction|FloattoStr00 (Math|Float|%(Float) _output_get 6e+01)))))

(fn ConstructionScript)

(fn FloattoStr00
  (params (number :type Float%20%28double-precision%29))
  (bind _returnvalue (Math|Float|Floor number))
  (bind _returnvalue_2 (Utilities|String|ToString(Integer) _returnvalue))
  (if (< _returnvalue 10)
    (return (Utilities|String|Append "0" _returnvalue_2))
    (else
      (return _returnvalue_2))))