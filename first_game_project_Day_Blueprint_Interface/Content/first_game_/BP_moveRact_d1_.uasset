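; Blueprint that moves a Cube component endlessly around a square path in its relative X-Z plane.
; Tick switches on the MoveType enum (Right, Up, Left, Down), stepping XR or ZUP and setting the cube's relative location.
; Each side hands over to the next state at its limit; steps are fixed per frame, so speed depends on frame rate.
; Unconnected Int and String switch nodes remain as reference.
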(event EventTick
  (params (DeltaSeconds :type Float%20%28single-precision%29))
  ;[0.15 0.15 0.15 0.5] 뱅뱅 도는 큐브의 코드
  (switch Utilities|FlowControl|Switch|SwitchonENUM_move_type (Variables|Default|Getmove_type)
    (:NewEnumerator0
      (Variables|Default|SetX+R (+ (Variables|Default|GetX+R) 1e+01))
      (Transformation|SetRelativeLocation (Variables|Default|GetCube) (Math|Vector|MakeVector (Variables|Default|GetX+R) 0.0 0.0) false false)
      (if (>= (Variables|Default|GetX+R) 2.5e+02)
        (Variables|Default|Setmove_type "NewEnumerator1")))
    (:NewEnumerator1
      (Variables|Default|SetZ+UP (+ (Variables|Default|GetZ+UP) 1e+01))
      (Transformation|SetRelativeLocation (Variables|Default|GetCube) (Math|Vector|MakeVector 2.5e+02 0.0 (Variables|Default|GetZ+UP)) false false)
      (if (>= (Variables|Default|GetZ+UP) 2.5e+02)
        (Variables|Default|Setmove_type "NewEnumerator2")))
    (:NewEnumerator2
      (bind _output_get (Variables|Default|SetX+R (+ (Variables|Default|GetX+R) -1e+01)))
      (Transformation|SetRelativeLocation (Variables|Default|GetCube) (Math|Vector|MakeVector _output_get 0.0 2.5e+02) false false)
      (if (<= (Variables|Default|GetX+R) 0.0)
        (Variables|Default|Setmove_type "NewEnumerator3")))
    (:NewEnumerator3
      (Variables|Default|SetZ+UP (+ (Variables|Default|GetZ+UP) -1e+01))
      (Transformation|SetRelativeLocation (Variables|Default|GetCube) (Math|Vector|MakeVector 0.0 0.0 (Variables|Default|GetZ+UP)) false false)
      (if (<= (Variables|Default|GetZ+UP) 0.0)
        (Variables|Default|Setmove_type "NewEnumerator0")))))

(fn ConstructionScript)