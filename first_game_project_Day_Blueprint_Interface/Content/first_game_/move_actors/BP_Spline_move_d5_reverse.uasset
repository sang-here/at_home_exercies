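; BP_Spline_move_d5_reverse is a moving-object Blueprint that carries a Cube back and forth along a spline.
; From BeginPlay, the OnNoff flag selects whether a timeline plays forward or in reverse.
; Timeline updates scale the spline length to a distance and set the Cube's world location there, without changing rotation.
; When the timeline finishes, it flips the flag and re-enters the branch, looping the motion continuously.
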(event EventBeginPlay
  ;[0.15 0.15 0.15 0.5] 계속해서 왔다가 돌아가는 스플라인 무브
  (if (Variables|Default|GetonNoff) :!label _label
    (bind _value (Timeline|타임라인 Play)
      (:Update
        (Transformation|SetWorldLocation (Variables|Default|GetCube) (.location (Spline|GetTransformatDistanceAlongSpline (Variables|Default|GetSpline) (* _value (Spline|GetSplineLength (Variables|Default|GetSpline))) "World" false)) false false))
      (:Finished
        (Variables|Default|SetonNoff (not (Variables|Default|GetonNoff)))
        (goto _label)))
    (else
      (Timeline|타임라인 Reverse))))

(fn ConstructionScript)