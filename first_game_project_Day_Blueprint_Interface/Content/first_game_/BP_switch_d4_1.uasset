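; BP_switch_d4_1 is a practice switch actor that triggers a spawn in another Blueprint when something overlaps its Cube.
; On begin overlap it prints the overlapped component, other actor and other component names for inspection, then calls DoSpawn on the referenced Abc.
; End overlap only prints an empty appended string.
; The construction script sets the TextRender label to the actor's own display name.
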(event OnComponentBeginOverlap(Cube)
  (params (OverlappedComponent :type Primitive%20Component%20Object%20Reference) (OtherActor :type Actor%20Object%20Reference) (OtherComp :type Primitive%20Component%20Object%20Reference) (OtherBodyIndex :type Integer) (bFromSweep :type Boolean) (SweepResult :type Hit%20Result%20Structure%20%28by%20ref%29))
  ;[0.15 0.15 0.15 0.5] 파라미터 확인 하는 법 / 스위치 만들기
  (Development|PrintString (Utilities|String|Append "begin overlap__" "_overlapped component:" (Utilities|GetDisplayName OverlappedComponent) "_other Actor :" (Utilities|GetDisplayName OtherActor) "_other comp:" (Utilities|GetDisplayName OtherComp)) true true "(R=0.000000,G=0.660000,B=1.000000,A=1.000000)" 7.0)
  ;[0.15 0.15 0.15 0.5] 다른 블루프린트와 연결점 만들기
  (Default|DoSpawn (Variables|Default|Getabc)))

(event OnComponentEndOverlap(Cube)
  (params (OverlappedComponent :type Primitive%20Component%20Object%20Reference) (OtherActor :type Actor%20Object%20Reference) (OtherComp :type Primitive%20Component%20Object%20Reference) (OtherBodyIndex :type Integer))
  ;[0.15 0.15 0.15 0.5 12] 드래그엔 그랍해서 액션 검색 및 생성
  (Development|PrintString (Utilities|String|Append "" "")))

(fn ConstructionScript
  (Rendering|Components|TextRender|SetText (Variables|Default|GetTextRender) (Utilities|Text|ToText(String) (Utilities|GetDisplayName self))))