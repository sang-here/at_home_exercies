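; Counter switch trigger that drives a set of moving test actors from overlaps with its Cube.
; Each begin overlap increments a text-rendered count wrapping at 10; even counts start every entry in Actors, and every end overlap stops them.
; Collapsed functions cast to four mover classes to toggle them; their Korean start/stop names are reversed relative to behavior.
; Inline custom-event copies and BP_PlayStop-based variants are not called here.
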(event OnComponentBeginOverlap(Cube)
  (params (OverlappedComponent :type Primitive%20Component%20Object%20Reference) (OtherActor :type Actor%20Object%20Reference) (OtherComp :type Primitive%20Component%20Object%20Reference) (OtherBodyIndex :type Integer) (bFromSweep :type Boolean) (SweepResult :type Hit%20Result%20Structure%20%28by%20ref%29))
  ;[0.15 0.15 0.15 0.5] 2,4,6,8 = T / 1,3,5,7,9 = F // a switch for everythiing - collapse to function
  ;;[0.15 0.15 0.15 0.5 12] 순서대로 하는 for loop 친구
  (Utilities|FlowControl|Sequence
    (:then_0
      (0|접촉시텍스트렌더가10까지1씩올라감))
    (:then_1
      ;;[0.15 0.15 0.15 0.5 12] 홀수라서 2로 나누면, 나머지가 1이라서 0보다 크면 T
      (if (not (> (Math|Integer|%(Integer) (Variables|Default|Getcount) 2) 0))
        (0|모든연결된액터들움직임멈추기)))))

(event OnComponentEndOverlap(Cube)
  (params (OverlappedComponent :type Primitive%20Component%20Object%20Reference) (OtherActor :type Actor%20Object%20Reference) (OtherComp :type Primitive%20Component%20Object%20Reference) (OtherBodyIndex :type Integer))
  ;[0.15 0.15 0.15 0.5] 2,4,6,8 = T / 1,3,5,7,9 = F // a switch for everythiing - collapse to function
  (0|모든연결된액터들움직이기시작))

(event Custom|CustomEvent
  (params (OverlappedComponent :type Primitive%20Component%20Object%20Reference) (OtherActor :type Actor%20Object%20Reference) (OtherComp :type Primitive%20Component%20Object%20Reference) (OtherBodyIndex :type Integer) (bFromSweep :type Boolean) (SweepResult :type Hit%20Result%20Structure%20%28by%20ref%29))
  ;[0.15 0.15 0.15 0.5] 2,4,6,8 = T / 1,3,5,7,9 = F // a switch for everythiing
  ;;[0.15 0.15 0.15 0.5 12] 순서대로 하는 for loop 친구
  (Utilities|FlowControl|Sequence
    (:then_0
      ;;[0.15 0.15 0.15 0.5] 지나가면 10까지 1씩 올라가는 텍스트
      ;;;[0.15 0.15 0.15 0.5 12] 닿을 때마다 +1
      (Variables|Default|Setcount (+ (Variables|Default|Getcount) 1))
      ;;;[0.15 0.15 0.15 0.5 12] text render에 텍스트 설정
      (Rendering|Components|TextRender|SetText (Variables|Default|GetTextRender) (Utilities|Text|ToText(Integer) (Variables|Default|Getcount)))
      ;;;[0.15 0.15 0.15 0.5 12] 10이 넘으면 0으로 변경
      (if (>= (Variables|Default|Getcount) 10)
        (Variables|Default|Setcount 0)))
    (:then_1
      ;;[0.15 0.15 0.15 0.5 12] 홀수라서 2로 나누면, 나머지가 1이라서 0보다 크면 T
      (if (not (> (Math|Integer|%(Integer) (Variables|Default|Getcount) 2) 0))
        (for _array_element (Variables|Default|GetActors)
          (bind _asbp_left_right_d_1_d_6 (Utilities|Casting|CastToBP_LeftRight_d1_d6 _array_element)
            (:then
              (Variables|/Game/first_game_/d6/BP_LeftRight_d1_d6.BP_LeftRight_d1_d6_C|SetIsPlay _asbp_left_right_d_1_d_6 true))
            (:CastFailed
              (bind _asbp_left_right_timeline_d_6 (Utilities|Casting|CastToBP_left_right_timeline_d6 _array_element)
                (:then
                  (Default|DoPlay _asbp_left_right_timeline_d_6))
                (:CastFailed
                  (bind _asbp_move_ract_2_d_3_d_6 (Utilities|Casting|CastToBP_moveRact2_d3_d6 _array_element)
                    (:then
                      (Variables|/Game/first_game_/d6/BP_moveRact2_d3_d6.BP_moveRact2_d3_d6_C|Setlever _asbp_move_ract_2_d_3_d_6 true))
                    (:CastFailed
                      (bind _asbp_move_left_timeline__d_4_d_6 (Utilities|Casting|CastToBP_move_left_Timeline__d4_d6 _array_element))
                      (Default|WeDoIt _asbp_move_left_timeline__d_4_d_6))))))))))))

(event Custom|CustomEvent_1
  (params (OverlappedComponent :type Primitive%20Component%20Object%20Reference) (OtherActor :type Actor%20Object%20Reference) (OtherComp :type Primitive%20Component%20Object%20Reference) (OtherBodyIndex :type Integer))
  ;[0.15 0.15 0.15 0.5] 2,4,6,8 = T / 1,3,5,7,9 = F // a switch for everythiing
  (for _array_element (Variables|Default|GetActors)
    (bind _asbp_left_right_d_1_d_6 (Utilities|Casting|CastToBP_LeftRight_d1_d6 _array_element)
      (:then
        (Variables|/Game/first_game_/d6/BP_LeftRight_d1_d6.BP_LeftRight_d1_d6_C|SetIsPlay _asbp_left_right_d_1_d_6 false))
      (:CastFailed
        (bind _asbp_left_right_timeline_d_6 (Utilities|Casting|CastToBP_left_right_timeline_d6 _array_element)
          (:then
            (Default|DoStop _asbp_left_right_timeline_d_6))
          (:CastFailed
            (bind _asbp_move_ract_2_d_3_d_6 (Utilities|Casting|CastToBP_moveRact2_d3_d6 _array_element)
              (:then
                (Variables|/Game/first_game_/d6/BP_moveRact2_d3_d6.BP_moveRact2_d3_d6_C|Setlever _asbp_move_ract_2_d_3_d_6 false))
              (:CastFailed
                (bind _asbp_move_left_timeline__d_4_d_6 (Utilities|Casting|CastToBP_move_left_Timeline__d4_d6 _array_element))
                (Default|WeDon'tDoIt _asbp_move_left_timeline__d_4_d_6)))))))))

(fn ConstructionScript)

(fn 모든연결된액터들움직이기시작
  (for _array_element (Variables|Default|GetActors)
    (bind _asbp_left_right_d_1_d_6 (Utilities|Casting|CastToBP_LeftRight_d1_d6 _array_element)
      (:then
        (Variables|/Game/first_game_/d6/BP_LeftRight_d1_d6.BP_LeftRight_d1_d6_C|SetIsPlay _asbp_left_right_d_1_d_6 false))
      (:CastFailed
        (bind _asbp_left_right_timeline_d_6 (Utilities|Casting|CastToBP_left_right_timeline_d6 _array_element)
          (:then
            (Default|DoStop _asbp_left_right_timeline_d_6))
          (:CastFailed
            (bind _asbp_move_ract_2_d_3_d_6 (Utilities|Casting|CastToBP_moveRact2_d3_d6 _array_element)
              (:then
                (Variables|/Game/first_game_/d6/BP_moveRact2_d3_d6.BP_moveRact2_d3_d6_C|Setlever _asbp_move_ract_2_d_3_d_6 false))
              (:CastFailed
                (bind _asbp_move_left_timeline__d_4_d_6 (Utilities|Casting|CastToBP_move_left_Timeline__d4_d6 _array_element))
                (Default|WeDon'tDoIt _asbp_move_left_timeline__d_4_d_6)))))))))

(fn 모든연결된액터들움직임멈추기
  (for _array_element (Variables|Default|GetActors)
    (bind _asbp_left_right_d_1_d_6 (Utilities|Casting|CastToBP_LeftRight_d1_d6 _array_element)
      (:then
        (Variables|/Game/first_game_/d6/BP_LeftRight_d1_d6.BP_LeftRight_d1_d6_C|SetIsPlay _asbp_left_right_d_1_d_6 true))
      (:CastFailed
        (bind _asbp_left_right_timeline_d_6 (Utilities|Casting|CastToBP_left_right_timeline_d6 _array_element)
          (:then
            (Default|DoPlay _asbp_left_right_timeline_d_6))
          (:CastFailed
            (bind _asbp_move_ract_2_d_3_d_6 (Utilities|Casting|CastToBP_moveRact2_d3_d6 _array_element)
              (:then
                (Variables|/Game/first_game_/d6/BP_moveRact2_d3_d6.BP_moveRact2_d3_d6_C|Setlever _asbp_move_ract_2_d_3_d_6 true))
              (:CastFailed
                (bind _asbp_move_left_timeline__d_4_d_6 (Utilities|Casting|CastToBP_move_left_Timeline__d4_d6 _array_element))
                (Default|WeDoIt _asbp_move_left_timeline__d_4_d_6)))))))))

(fn 접촉시텍스트렌더가10까지1씩올라감
  ;[0.15 0.15 0.15 0.5] 지나가면 10까지 1씩 올라가는 텍스트
  (지나가면10까지1씩올라가는텍스트|변수가1씩올라감)
  (지나가면10까지1씩올라가는텍스트|그변수는10이될수없어요)
  (지나가면10까지1씩올라가는텍스트|설정된변수가텍스트렌더에적용되요))

(fn 짝수면F값/홀수면T값
  ;[0.15 0.15 0.15 0.5 12] 홀수라서 2로 나누면, 나머지가 1이라서 0보다 크면 T
  (if (> (Math|Integer|%(Integer) (Variables|Default|Getcount) 2) 0)
    _))

(fn 변수가1씩올라감
  ;[0.15 0.15 0.15 0.5 12] 닿을 때마다 +1
  (Variables|Default|Setcount (+ (Variables|Default|Getcount) 1)))

(fn 설정된변수가텍스트렌더에적용되요
  ;[0.15 0.15 0.15 0.5 12] text render에 텍스트 설정
  (Rendering|Components|TextRender|SetText (Variables|Default|GetTextRender) (Utilities|Text|ToText(Integer) (Variables|Default|Getcount))))

(fn 그변수는10이될수없어요
  ;[0.15 0.15 0.15 0.5 12] 10이 넘으면 0으로 변경
  (if (>= (Variables|Default|Getcount) 10)
    (Variables|Default|Setcount 0)))

(fn Interface모든연결된액터들움직이기시작0
  (for _array_element (Variables|Default|GetActors)
    (bind _asbp_play_stop (Utilities|Casting|CastToBP_PlayStop _array_element))
    (Default|DoPlayandStop0 _asbp_play_stop true)))

(fn Interface모든연결된액터들움직임멈추기0
  (for _array_element (Variables|Default|GetActors)
    (bind _asbp_play_stop (Utilities|Casting|CastToBP_PlayStop _array_element))
    (Default|DoPlayandStop0 _asbp_play_stop false)))

(fn DoPlayandStop0
  (params (DoPlay :type Boolean))
  (return false))