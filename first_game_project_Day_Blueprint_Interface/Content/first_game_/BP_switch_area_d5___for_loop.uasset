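; A practice trigger-switch actor that fires two spawners when something overlaps its Cube, built to experiment with For Loop nodes.
; On begin overlap, two sequential loops call DoSpawn ten times on Spawner1, then five times on Spawner2, printing each index and a completion message.
; End overlap prints an empty string, and disconnected test nodes remain in the graph.
; The construction script labels the TextRender with the actor's display name.
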(event OnComponentBeginOverlap(Cube)
  (params (OverlappedComponent :type Primitive%20Component%20Object%20Reference) (OtherActor :type Actor%20Object%20Reference) (OtherComp :type Primitive%20Component%20Object%20Reference) (OtherBodyIndex :type Integer) (bFromSweep :type Boolean) (SweepResult :type Hit%20Result%20Structure%20%28by%20ref%29))
  ;[0.15 0.15 0.15 0.5] 파라미터 확인 하는 법 / 스위치 만들기
  ;[0.15 0.15 0.15 0.5] 실습/ 5번과 10번을 한번에 산출하는 스위치 만들기
  (for _index (range 1 10)
    (Development|PrintString (Utilities|String|ToString(Integer) _index))
    (Default|DoSpawn (Variables|Default|Getspawner_1)))
  (Development|PrintString "completed")
  (for _index_2 (range 1 5)
    (Development|PrintString (Utilities|String|ToString(Integer) _index_2))
    (Default|DoSpawn (Variables|Default|Getspawner_2)))
  (Development|PrintString "completed"))

(event OnComponentEndOverlap(Cube)
  (params (OverlappedComponent :type Primitive%20Component%20Object%20Reference) (OtherActor :type Actor%20Object%20Reference) (OtherComp :type Primitive%20Component%20Object%20Reference) (OtherBodyIndex :type Integer))
  ;[0.15 0.15 0.15 0.5 12] 드래그엔 그랍해서 액션 검색 및 생성
  (Development|PrintString (Utilities|String|Append "" "")))

(fn ConstructionScript
  (Rendering|Components|TextRender|SetText (Variables|Default|GetTextRender) (Utilities|Text|ToText(String) (Utilities|GetDisplayName self))))