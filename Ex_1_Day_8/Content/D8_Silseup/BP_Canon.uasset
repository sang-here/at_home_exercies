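; BP_Canon is a cannon actor that fires BP_CanonBall projectiles and reports each shot to the player HUD.
; Overlapping its cube prints a "Press F to shoot" debug prompt; input is handled outside this graph.
; CanonBallon spawns the ball at the Arrow's transform, then calls BP_Hud on every PlayerController to update the widget.
; A separate switch event waits briefly before triggering a second HUD message.
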(event OnComponentBeginOverlap(Cube1)
  (params (OverlappedComponent :type Primitive%20Component%20Object%20Reference) (OtherActor :type Actor%20Object%20Reference) (OtherComp :type Primitive%20Component%20Object%20Reference) (OtherBodyIndex :type Integer) (bFromSweep :type Boolean) (SweepResult :type Hit%20Result%20Structure%20%28by%20ref%29))
  (Development|PrintString "Press_F_to_shoot"))

(event EventFromBPISwitchCanonWaitAfterShoot
  (Development|PrintString "delay")
  (Utilities|FlowControl|Delay 1.0)
  (Hud&Widget|2ShowStrThruhud&Widget))

(event EventCanonBallon
  (Development|PrintString "Canon_fired")
  (CallFunction|SpawnCanonBallatRightPosition)
  (Utilities|FlowControl|Sequence
    (:then_0
      (Hud&Widget|1ShowStrThruhud&Widget))
    (:then_1
      (CallFunction|AddCanoninWidget))))

(fn ConstructionScript)

(fn 1ShowStrThruhud&Widget
  (bind _outactors (Actor|GetAllActorsOfClass "/Script/Engine.PlayerController"))
  (for _array_element _outactors
    (bind _asbp_hud (Utilities|Casting|CastToBP_Hud (HUD|GetHUD _array_element)))
    (Default|InBPHud1CanonSrtFncttoWidgetHud _asbp_hud)))

(fn 2ShowStrThruhud&Widget
  (bind _outactors (Actor|GetAllActorsOfClass "/Script/Engine.PlayerController"))
  (for _array_element _outactors
    (bind _asbp_hud (Utilities|Casting|CastToBP_Hud (HUD|GetHUD _array_element)))
    (Default|InBPHud2CanonSrtFncttoWidgetHud _asbp_hud)))

(fn SpawnCanonBallatRightPosition
  (bind _arrow (Variables|Default|GetArrow))
  (Game|SpawnActorfromClass "/Game/D8_Silseup/BP_CanonBall.BP_CanonBall_C" (Math|Transform|MakeTransform (Transformation|GetWorldLocation _arrow) (Transformation|GetWorldRotation _arrow) "1.000000,1.000000,1.000000") "Undefined" "MultiplyWithRoot" 0 0))

(fn AddCanoninWidget
  (bind _outactors (Actor|GetAllActorsOfClass "/Script/Engine.PlayerController"))
  (for _array_element _outactors
    (bind _asbp_hud (Utilities|Casting|CastToBP_Hud (HUD|GetHUD _array_element)))
    (Default|InBPHudAddCanonFnctfromBPCanontoWidgetHud _asbp_hud)))