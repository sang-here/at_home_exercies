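; BP_Counter_d6 is a countdown counter Blueprint that shows a number which drops each time something overlaps its Cube.
; Count starts at 9 on BeginPlay, and each Cube begin-overlap subtracts one without filtering the overlapping actor.
; Tick writes Count to the TextRender every frame, then resets it to 9 once it reaches zero or below.
; An unconnected count-up variant that wraps at ten remains in the graph but never runs.
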(event OnComponentBeginOverlap(Cube)
  (params (OverlappedComponent :type Primitive%20Component%20Object%20Reference) (OtherActor :type Actor%20Object%20Reference) (OtherComp :type Primitive%20Component%20Object%20Reference) (OtherBodyIndex :type Integer) (bFromSweep :type Boolean) (SweepResult :type Hit%20Result%20Structure%20%28by%20ref%29))
  ;[0.15 0.15 0.15 0.5] 이렇게도 할  수 있지만, 실무적으로는 변수의 값을 변경하지 않고 유지하면서, while using the existing value, you build your own codes
  ;;[0.15 0.15 0.15 0.5] 지나가면 9에서부터 1씩 내려가는 텍스트
  ;;;[0.15 0.15 0.15 0.5 12] 닿을 때마다 -1
  (Variables|Default|Setcount (- (Variables|Default|Getcount) 1)))

(event EventTick
  (params (DeltaSeconds :type Float%20%28single-precision%29))
  ;[0.15 0.15 0.15 0.5] 이렇게도 할  수 있지만, 실무적으로는 변수의 값을 변경하지 않고 유지하면서, while using the existing value, you build your own codes
  ;;[0.15 0.15 0.15 0.5] 지나가면 9에서부터 1씩 내려가는 텍스트
  ;;;[0.15 0.15 0.15 0.5 12] text render에 텍스트 설정
  (Rendering|Components|TextRender|SetText (Variables|Default|GetTextRender) (Utilities|Text|ToText(Integer) (Variables|Default|Getcount)))
  ;;;[0.15 0.15 0.15 0.5 12] 0이 되면 9로 변경
  (if (<= (Variables|Default|Getcount) 0)
    (Variables|Default|Setcount 9)))

(event EventBeginPlay
  ;[0.15 0.15 0.15 0.5] 이렇게도 할  수 있지만, 실무적으로는 변수의 값을 변경하지 않고 유지하면서, while using the existing value, you build your own codes
  ;;[0.15 0.15 0.15 0.5] 지나가면 9에서부터 1씩 내려가는 텍스트
  ;;;[0.15 0.15 0.15 0.5 12] 9로 시작
  (Variables|Default|Setcount 9))

(fn ConstructionScript)