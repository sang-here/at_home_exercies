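; BP_CountBox is a counter box that shows a running count on its TextRender.
; Each Counton event prints a debug message, increments ForTextRender and writes it to the text, wrapping back to one after ten.
; An "off" debug print is present but never runs, and the construction script is empty.
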(event EventCounton
  (Development|PrintString "CounterBox_is_on")
  (if (>= (Variables|Default|GetForTextRender) 10)
    (Variables|Default|SetForTextRender 0))
  (Variables|Default|SetForTextRender (+ (Variables|Default|GetForTextRender) 1))
  (Rendering|Components|TextRender|SetText (Variables|Default|GetTextRender) (Utilities|Text|ToText(Integer) (Variables|Default|GetForTextRender))))

(fn ConstructionScript)