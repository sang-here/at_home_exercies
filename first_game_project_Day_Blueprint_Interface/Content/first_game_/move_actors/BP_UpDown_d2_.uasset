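; An actor Blueprint that bounces its Cone component up and down in an endless loop.
; Each Tick steps a stored Z value by a fixed amount and applies it as the cone's relative location, flipping a direction flag at the upper and lower limits.
; The step ignores delta time, so the speed depends on frame rate.
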(event EventTick
  (params (DeltaSeconds :type Float%20%28single-precision%29))
  ;[0.15 0.15 0.15 0.5] 위아래로 움직이는 코드
  (if (Variables|Default|GetIs_Move_up)
    (Variables|Default|SetLoc_Z (+ (Variables|Default|GetLoc_Z) 5.0))
    (Transformation|SetRelativeLocation (Variables|Default|GetCone) (Math|Vector|MakeVector 0.0 0.0 (Variables|Default|GetLoc_Z)) false false)
    (if (>= (Variables|Default|GetLoc_Z) 2.5e+02)
      (Variables|Default|SetIs_Move_up false))
    (else
      (Variables|Default|SetLoc_Z (+ (Variables|Default|GetLoc_Z) -5.0))
      (Transformation|SetRelativeLocation (Variables|Default|GetCone) (Math|Vector|MakeVector 0.0 0.0 (Variables|Default|GetLoc_Z)) false false)
      (if (<= (Variables|Default|GetLoc_Z) 0.0)
        (Variables|Default|SetIs_Move_up true)))))

(fn ConstructionScript)