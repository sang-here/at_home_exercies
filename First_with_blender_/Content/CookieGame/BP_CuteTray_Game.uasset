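; BP_CuteTray_Game is a cookie-game tray actor that moves forward with a small hop and can turn sideways.
; A looping timeline from BeginPlay sets its relative X and Z, restarting the path each cycle.
; WorldLocationLimit checks a square world boundary and fires an event that randomly plays a left or right 90-degree yaw timeline.
; Nothing in this graph calls that check, and debug prints remain.
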(event Custom|WorldLocationLimitEvent
  ;[0.15 0.15 0.15 0.5] 뭐에 막히면 왼 혹은 오른 으로 turn 90 degree
  (Development|PrintString "Hello")
  (if (Math|Random|RandomBool)
    (bind _newtrack_0 (Timeline|Turn90Degree Play)
      (:Update
        (Transformation|SetRelativeRotation (Variables|Default|GetCuteTray) (Math|Rotator|MakeRotator 0.0 0.0 (* _newtrack_0 9e+01)) false false)))
    (else
      (bind _newtrack_0_2 (Timeline|Turn90Degree0 Play)
        (:Update
          (Transformation|SetRelativeRotation (Variables|Default|GetCuteTray) (Math|Rotator|MakeRotator 0.0 0.0 (* _newtrack_0_2 -9e+01)) false false))))))

(event EventBeginPlay
  ;[0.15 0.15 0.15 0.5] 앞으로 가다가 5~6초사이 점프 살짝
  (bind _newtrack_0 (Timeline|GoForwardTill6SecsButJunpAt5 Play)
    (:Update
      (Transformation|SetRelativeLocation (Variables|Default|GetCuteTray) (Math|Vector|MakeVector (* (.x _newtrack_0) 2e+02) 0.0 (* (.z _newtrack_0) 2e+01)) false false))
    (:Finished
      (Timeline|GoForwardTill6SecsButJunpAt5 PlayFromStart))))

(fn ConstructionScript)

(fn WorldLocationLimit
  (bind _cutetray (Variables|Default|GetCuteTray))
  (bind _returnvalue (Transformation|GetWorldLocation _cutetray))
  (if (Math|Boolean|ORBoolean (<= (.x _returnvalue) -1.5e+03) (>= (.x _returnvalue) 1.5e+03) (<= (.y _returnvalue) -1.5e+03) (>= (.y _returnvalue) 1.5e+03))
    (Development|PrintString "Hello0" true true "(R=0.000000,G=0.660000,B=1.000000,A=1.000000)" 5e+01)
    (CallFunction|WorldLocationLimitEvent)))