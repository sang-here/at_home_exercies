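; Moving actor Blueprint that loops its Sphere component around a square path in the relative X-Z plane while the Lever flag is true.
; Tick switches on the NewVar direction enum, calling one function per side that steps the Sphere and advances the direction at its limit.
; Steps are fixed per frame, so speed depends on frame rate.
; CustomEvent holds the same logic unfolded and is not called here.
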(event Custom|CustomEvent
  (params (DeltaSeconds :type Float%20%28single-precision%29))
  ;[0.15 0.15 0.15 0.5 12] D6(reference)
  (if (Variables|Default|Getlever)
    ;[0.15 0.15 0.15 0.5] 뱅뱅 도는 코드 (신버전)
    (switch Utilities|FlowControl|Switch|SwitchonEN_Move_type_2 (Variables|Default|GetNewVar)
      (:NewEnumerator0
        (Transformation|AddRelativeLocation (Variables|Default|GetSphere) (Math|Vector|MakeVector 0.0 0.0 1e+01) false false)
        (if (>= (.z (Variables|/Script/Engine.SceneComponent|GetRelativeLocation (Variables|Default|GetSphere))) 2.5e+02)
          (Variables|Default|SetNewVar "NewEnumerator1")))
      (:NewEnumerator1
        (Transformation|AddRelativeLocation (Variables|Default|GetSphere) (Math|Vector|MakeVector 1e+01 0.0 0.0) false false)
        (if (>= (.x (Variables|/Script/Engine.SceneComponent|GetRelativeLocation (Variables|Default|GetSphere))) 2.5e+02)
          (Variables|Default|SetNewVar "NewEnumerator2")))
      (:NewEnumerator2
        (Transformation|AddRelativeLocation (Variables|Default|GetSphere) (Math|Vector|MakeVector 0.0 0.0 -1e+01) false false)
        (if (<= (.z (Variables|/Script/Engine.SceneComponent|GetRelativeLocation (Variables|Default|GetSphere))) 0.0)
          (Variables|Default|SetNewVar "NewEnumerator3")))
      (:NewEnumerator3
        (Transformation|AddRelativeLocation (Variables|Default|GetSphere) (Math|Vector|MakeVector -1e+01 0.0 0.0) false false)
        (if (<= (.x (Variables|/Script/Engine.SceneComponent|GetRelativeLocation (Variables|Default|GetSphere))) 0.0)
          (Variables|Default|SetNewVar "NewEnumerator0"))))))

(event EventTick
  (params (DeltaSeconds :type Float%20%28single-precision%29))
  ;[0.15 0.15 0.15 0.5] 뱅뱅 도는 코드 (신버전) / 함수로 접기
  ;;[0.15 0.15 0.15 0.5 12] D6(reference)
  (if (Variables|Default|Getlever)
    (switch Utilities|FlowControl|Switch|SwitchonEN_Move_type_2 (Variables|Default|GetNewVar)
      (:NewEnumerator0
        (CallFunction|250까지Z값10씩추가후Right산출))
      (:NewEnumerator1
        (CallFunction|250까지X값10씩추가후Down산출))
      (:NewEnumerator2
        (CallFunction|0까지Z값-10씩절감후Left산출))
      (:NewEnumerator3
        (CallFunction|0까지X값-10씩절감후Up산출)))))

(fn ConstructionScript)

(fn 250까지Z값10씩추가후Right산출
  (Transformation|AddRelativeLocation (Variables|Default|GetSphere) (Math|Vector|MakeVector 0.0 0.0 1e+01) false false)
  (if (>= (.z (Variables|/Script/Engine.SceneComponent|GetRelativeLocation (Variables|Default|GetSphere))) 2.5e+02)
    (Variables|Default|SetNewVar "NewEnumerator1")))

(fn 250까지X값10씩추가후Down산출
  (Transformation|AddRelativeLocation (Variables|Default|GetSphere) (Math|Vector|MakeVector 1e+01 0.0 0.0) false false)
  (if (>= (.x (Variables|/Script/Engine.SceneComponent|GetRelativeLocation (Variables|Default|GetSphere))) 2.5e+02)
    (Variables|Default|SetNewVar "NewEnumerator2")))

(fn 0까지Z값-10씩절감후Left산출
  (Transformation|AddRelativeLocation (Variables|Default|GetSphere) (Math|Vector|MakeVector 0.0 0.0 -1e+01) false false)
  (if (<= (.z (Variables|/Script/Engine.SceneComponent|GetRelativeLocation (Variables|Default|GetSphere))) 0.0)
    (Variables|Default|SetNewVar "NewEnumerator3")))

(fn 0까지X값-10씩절감후Up산출
  (Transformation|AddRelativeLocation (Variables|Default|GetSphere) (Math|Vector|MakeVector -1e+01 0.0 0.0) false false)
  (if (<= (.x (Variables|/Script/Engine.SceneComponent|GetRelativeLocation (Variables|Default|GetSphere))) 0.0)
    (Variables|Default|SetNewVar "NewEnumerator0")))