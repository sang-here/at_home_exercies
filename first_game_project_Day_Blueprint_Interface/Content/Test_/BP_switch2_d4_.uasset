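; Apple switch actor that counts overlaps on its Sphere component and requests an apple spawn on each one.
; Each overlap increments HowManyApples and prints a message for the first apple, later apples, or a "no more apples" limit past ten.
; Every branch then calls AppleSpawn on the Apple1 reference, so the limit changes only the printed text and does not stop spawning.
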(event OnComponentBeginOverlap(Sphere)
  (params (OverlappedComponent :type Primitive%20Component%20Object%20Reference) (OtherActor :type Actor%20Object%20Reference) (OtherComp :type Primitive%20Component%20Object%20Reference) (OtherBodyIndex :type Integer) (bFromSweep :type Boolean) (SweepResult :type Hit%20Result%20Structure%20%28by%20ref%29))
  ;[0.15 0.15 0.15 0.5] 사과 스위치 만들기
  (Variables|Default|Sethow_many_apples (+ (Variables|Default|GetHow_Many_Apples) 1.0))
  (if (== 1.0 (Variables|Default|GetHow_Many_Apples))
    (Development|PrintString (Utilities|String|Append (Utilities|String|ToString(Float) (Variables|Default|GetHow_Many_Apples)) "_apple" "_checked") true true "(R=0.000000,G=0.660000,B=1.000000,A=1.000000)" 5.0)
    (elif (>= (Variables|Default|GetHow_Many_Apples) 10.5)
      (Development|PrintString (Utilities|String|Append "sorry_" "no_more_apples" "_checked") true true "(R=0.000000,G=0.660000,B=1.000000,A=1.000000)" 5.0)
      (else
        (Development|PrintString (Utilities|String|Append (Utilities|String|ToString(Float) (Variables|Default|GetHow_Many_Apples)) "_apples given" "_checked") true true "(R=0.000000,G=0.660000,B=1.000000,A=1.000000)" 5.0))))
  (Default|AppleSpawn (Variables|Default|Getapple1)))

(event Collision|EventActorBeginOverlap
  (params (OtherActor :type Actor%20Object%20Reference))
  ;[0.15 0.15 0.15 0.5] 사과 스위치 만들기
)

(fn ConstructionScript)