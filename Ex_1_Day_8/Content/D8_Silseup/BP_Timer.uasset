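; Timer Blueprint that counts elapsed time and shows it as minutes and seconds on a TextRender.
; While TimerOnOff is true, Tick accumulates delta seconds, and duplicated helper graphs derive floored minutes and seconds.
; Four sequenced branches handle zero-padding, but their comparisons skip updates at second 9 before minute 10 and throughout minute 9.
; The last branch's seconds check is unwired, so from minute 10 it overwrites padded seconds with unpadded ones.
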(event EventTick
  (params (DeltaSeconds :type Float%20%28single-precision%29))
  (bind _returnvalue (|minute_2))
  (bind _returnvalue_2 (|second_2))
  (bind _returnvalue_3 (|minute_2_2))
  (bind _returnvalue_4 (|second_2_2))
  (bind _returnvalue_5 (|minute))
  (bind _returnvalue_6 (|second))
  (bind _returnvalue_7 (|minute_2_2_2))
  (if (Variables|Default|GetTimerOnOff)
    (Variables|Default|SetTotalDeltaSeconds (+ (Variables|Default|GetTotalDeltaSeconds) (* DeltaSeconds 1.0)))
    (Utilities|FlowControl|Sequence
      (:then_0
        (if (< _returnvalue_6 9)
          (if (< _returnvalue_5 9)
            (Rendering|Components|TextRender|SetText (Variables|Default|GetTextRender) (Utilities|Text|ToText(String) (Utilities|String|Append "0" (Utilities|String|ToString(Integer) _returnvalue_5) ":" "0" (Utilities|String|ToString(Integer) _returnvalue_6)))))))
      (:then_1
        (if (>= _returnvalue_2 10)
          (if (< _returnvalue 9)
            (Rendering|Components|TextRender|SetText (Variables|Default|GetTextRender) (Utilities|Text|ToText(String) (Utilities|String|Append "0" (Utilities|String|ToString(Integer) _returnvalue) ":" (Utilities|String|ToString(Integer) _returnvalue_2)))))))
      (:then_2
        (if (< _returnvalue_4 9)
          (if (>= _returnvalue_3 10)
            (Rendering|Components|TextRender|SetText (Variables|Default|GetTextRender) (Utilities|Text|ToText(String) (Utilities|String|Append (Utilities|String|ToString(Integer) _returnvalue_3) ":" "0" (Utilities|String|ToString(Integer) _returnvalue_4)))))))
      (:then_3
        (if true
          (if (>= _returnvalue_7 10)
            (Rendering|Components|TextRender|SetText (Variables|Default|GetTextRender) (Utilities|Text|ToText(String) (Utilities|String|Append (Utilities|String|ToString(Integer) _returnvalue_7) ":" (Utilities|String|ToString(Integer) (|second_2_2_2)))))))))))

(fn ConstructionScript)