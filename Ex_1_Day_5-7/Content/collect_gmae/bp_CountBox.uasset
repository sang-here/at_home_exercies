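; A counter box Blueprint that displays how many fruits have been collected on a TextRender component.
; The plusInfo and minusInfo events raise or lower the fruit count by one, print a debug string and refresh the displayed text.
; The Info event is empty, and a disconnected copy of the increment logic remains unused in the graph.
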(event Custom|Info)

(event Custom|minusInfo
  (Development|PrintString "Info_-on")
  (Variables|Default|SetHowManyFruitsDidYouHave (+ (Variables|Default|GetHowManyFruitsDidYouHave) -1))
  (Rendering|Components|TextRender|SetText (Variables|Default|GetTextRender) (Utilities|Text|ToText(Integer) (Variables|Default|GetHowManyFruitsDidYouHave))))

(event Custom|plusInfo
  (Development|PrintString "Info_+on")
  (Variables|Default|SetHowManyFruitsDidYouHave (+ (Variables|Default|GetHowManyFruitsDidYouHave) 1))
  (Rendering|Components|TextRender|SetText (Variables|Default|GetTextRender) (Utilities|Text|ToText(Integer) (Variables|Default|GetHowManyFruitsDidYouHave))))

(fn ConstructionScript)